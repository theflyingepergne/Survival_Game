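; BP_Camera is a shared camera that keeps all active players in view once the game starts.
; GameStarted stores the active players map and, on the first call, fades the camera in from black.
; Each tick it lerps a Sphere toward the players' average location and sets the spring arm length to the largest pairwise player distance, clamped between minimum and maximum values.
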(event EventTick
  (params (DeltaSeconds :type Float%20%28single-precision%29))
  (if (Variables|Default|GetbGameStarted)
    (CallFunction|UpdateCameraMovement)
    (CallFunction|UpdateSpringArmLength)))

(fn ConstructionScript)

(fn GameStarted
  (params (ActivePlayersMap :type Map%20of%20Integers%20to%20Objects))
  (Variables|Default|SetActivePlayersMap ActivePlayersMap)
  (if (not (Variables|Default|GetbGameStarted))
    (Variables|Default|SetbGameStarted true)
    (CameraFades|StartCameraFade :self (Game|GetPlayerCameraManager 0) :FromAlpha 1.0 :Duration 0.5)))

(fn UpdateCameraMovement
  (Variables|Default|SetPreviousLocation (Transformation|GetWorldLocation (Variables|Default|GetSphere)))
  (bind _values (Utilities|Map|Values (Variables|Default|GetActivePlayersMap)))
  (bind _returnvalue (Class|GameplayStatics|GetActorArrayAverageLocation _values))
  (Transformation|SetWorldLocation (Variables|Default|GetSphere) (Math|Vector|Lerp(Vector) (Variables|Default|GetPreviousLocation) _returnvalue (Variables|Default|GetMoveSpeed)) false false))

(fn UpdateSpringArmLength
  (bind _values (Utilities|Map|Values (Variables|Default|GetActivePlayersMap)))
  (bind _output_get (LocalVariables|SetActivePlayersLoc _values))
  (for (_array_element _array_index) _output_get
    (Variables|Default|SetPlayer _array_element)
    (for _index (range (+ _array_index 1) (- (Utilities|Array|Length (LocalVariables|GetActivePlayersLoc)) 1))
      (Utilities|Array|Add (Variables|Default|GetDistance) (Transformation|GetDistanceTo (Variables|Default|GetPlayer) (Utilities|Array|Get(acopy) (LocalVariables|GetActivePlayersLoc) _index)))))
  (Variables|/Script/Engine.SpringArmComponent|SetTargetArmLength (Variables|Default|GetSpringArm) (Math|Float|Clamp(Float) (.MaxValue (Math|Float|MaxOfFloatArray (Variables|Default|GetDistance))) (Variables|Default|GetMinArmLength) (Variables|Default|GetMaxArmLength)))
  (Utilities|Array|Clear (Variables|Default|GetDistance)))