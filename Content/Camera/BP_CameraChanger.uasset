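; BP_CameraChanger is a trigger volume that rotates the game camera to match its CameraForPreview component while something overlaps it.
; On the first overlap it gets the camera from the GameMode and caches its default rotation.
; A timeline lerps the camera root's world rotation toward the preview's and reverses on end overlap, with BlendSpeedIn setting the play rate both ways.
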(event OnComponentBeginOverlap(TriggerBox)
  (params (OverlappedComponent :type Primitive%20Component%20Object%20Reference) (OtherActor :type Actor%20Object%20Reference) (OtherComp :type Primitive%20Component%20Object%20Reference) (OtherBodyIndex :type Integer) (bFromSweep :type Boolean) (SweepResult :type Hit%20Result%20Structure%20%28by%20ref%29))
  (Variables|Default|GetCameraRef
    (:then
      _)
    (:else
      (bind _camera (Class|BPIGameMode|GetCamera(Message) (Game|GetGameMode)))
      (bind _output_get (Variables|Default|SetCameraRef _camera))
      (Variables|Default|SetCameraDefaultRot (Transformation|GetWorldRotation (Variables|/Script/Engine.Actor|GetRootComponent _output_get)))))
  (Components|Timeline|SetPlayRate (Variables|Default|GetCameraChangeSpeed) (Variables|Default|GetBlendSpeed_In))
  (bind _alpha (Timeline|CameraChangeSpeed Play)
    (:Update
      (Transformation|SetWorldRotation (Variables|/Script/Engine.Actor|GetRootComponent (Variables|Default|GetCameraRef)) (Math|Rotator|Lerp(Rotator) (Variables|Default|GetCameraDefaultRot) (Transformation|GetWorldRotation (Variables|Default|GetCamera%28ForPreview%29)) _alpha) false false))))

(event OnComponentEndOverlap(TriggerBox)
  (params (OverlappedComponent :type Primitive%20Component%20Object%20Reference) (OtherActor :type Actor%20Object%20Reference) (OtherComp :type Primitive%20Component%20Object%20Reference) (OtherBodyIndex :type Integer))
  (Components|Timeline|SetPlayRate (Variables|Default|GetCameraChangeSpeed) (Variables|Default|GetBlendSpeed_In))
  (bind _alpha (Timeline|CameraChangeSpeed Reverse)
    (:Update
      (Transformation|SetWorldRotation (Variables|/Script/Engine.Actor|GetRootComponent (Variables|Default|GetCameraRef)) (Math|Rotator|Lerp(Rotator) (Variables|Default|GetCameraDefaultRot) (Transformation|GetWorldRotation (Variables|Default|GetCamera%28ForPreview%29)) _alpha) false false))))

(fn ConstructionScript)