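; Per-player input receiver that handles joining the game and choosing a character from a menu.
; Outside gameplay, JoinGame either asks the game mode to display character select or, if the menu exists, confirms the choice.
; Confirming stores the choice in the game instance, requests a spawn from the game mode and removes the menu, while left and right inputs cycle characters.
; Communication uses interface messages, and its own interface functions are stubs.
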(event EventBeginPlay
  (Class|BPIGameMode|GetIsStartingLevel(Message) (Game|GetGameMode)))

(event Input|ActionEvents|InputActionMenuLeft
  (params (Key :type Key%20Structure :default "None"))
  (:Pressed
    (bind _charactermenuref (Variables|Default|GetCharacterMenuRef)
      (:then
        (Default|SwitchCharacter _charactermenuref -1))
      (:else))))

(event Input|ActionEvents|InputActionMenuRight
  (params (Key :type Key%20Structure :default "None"))
  (:Pressed
    (bind _charactermenuref (Variables|Default|GetCharacterMenuRef)
      (:then
        (Default|SwitchCharacter _charactermenuref 1))
      (:else))))

(event Input|ActionEvents|InputActionJoinGame
  (params (Key :type Key%20Structure :default "None"))
  (:Pressed
    (bind _isingame (Class|BPIGameMode|GetIsinGame(Message) (Game|GetGameMode)))
    (if (not _isingame)
      (Variables|Default|GetCharacterMenuRef
        (:then
          (Class|BPIGameInstance|SetCharacterChoice(Message) (Game|GetGameInstance) (Variables|Default|GetPlayerIndex) (Variables|/Game/UI/PreGame/WBP_CharacterSelect.WBP_CharacterSelect_C|GetCharacterChoice (Variables|Default|GetCharacterMenuRef)))
          (bind _characterchoice (Class|BPIGameInstance|GetCharacterChoice(Message) (Game|GetGameInstance) (Variables|Default|GetPlayerIndex)))
          (Class|BPIGameMode|SpawnPlayer(Message) (Game|GetGameMode) (Variables|Default|GetPlayerIndex) _characterchoice self)
          (Widget|RemovefromParent (Variables|Default|GetCharacterMenuRef))
          (Variables|Default|SetCharacterMenuRef 0))
        (:else
          (Class|BPIGameMode|DisplayCharacterSelect(Message) (Game|GetGameMode) (Variables|Default|GetPlayerIndex)))))))

(fn ConstructionScript)

(fn DisplayCharacterSelect
  (params (CurrentPlayerIndex :type Integer))
  (return false))

(fn GetIsinGame
  (return false))

(fn GetIsStartingLevel
  (return false))

(fn SpawnPlayer
  (params (CurrentPlayerIndex :type Integer) (CharacterChoice :type Integer) (InputReceiver :type BP%20Input%20Receiver%20Object%20Reference))
  (return false))

(fn StartGame
  (return false))