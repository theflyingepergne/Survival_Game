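; Core game mode for a local multiplayer game: spawns the shared camera, players and UI, and tracks deaths.
; Starting levels create input receivers at tagged PlayerStarts for menu-driven character select.
; Other levels respawn players from GameInstance data at a matching custom-tag start (else the first non-"Cust_" start) and start immediately.
; Death and revive events update a count; when all players die, it fades out and shows the death screen.
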(event Custom|OnPlayerDied
  ;[0.05127 0.05127 0.05127] Handle Player death
  (bind _output_get (Variables|Default|SetPlayersDeadCount (+ (Variables|Default|GetPlayersDeadCount) 1)))
  (Development|PrintString (Utilities|String|ToString(Integer) _output_get))
  (Development|PrintString "Player death count:")
  (bind _numplayers (Class|BPIGameInstance|GetPlayerMap(Message) (Game|GetGameInstance)))
  (if (>= (Variables|Default|GetPlayersDeadCount) _numplayers)
    (Utilities|FlowControl|Delay 2.0)
    (Default|CallFadeinGameHUD)
    (CameraFades|StartCameraFade :self (Game|GetPlayerCameraManager 0) :ToAlpha 1.0 :Duration 1.0 :bHoldWhenFinished true)
    (Utilities|FlowControl|Delay 2.0)
    (bind _returnvalue (UserInterface|CreateWidget "/Game/Maps/Level_End/WBP_End_Death.WBP_End_Death_C"))
    (UserInterface|Viewport|AddtoViewport _returnvalue 0)
    (Widget|SetFocus _returnvalue)))

(event EventBeginPlay
  (CallFunction|GetPlayerStartPoints)
  ;[0.05127 0.05127 0.05127] Spawn camera
  (bind _returnvalue (CallFunction|DoCustomSpawn))
  (bind _returnvalue_2 (Game|SpawnActorfromClass "/Game/Camera/BP_Camera.BP_Camera_C" (Math|Transform|MakeTransform (.Location (Math|Transform|BreakTransform _returnvalue))) "Undefined" 0 0))
  (Variables|Default|SetCameraRef _returnvalue_2)
  ;[0.05127 0.05127 0.05127] Spawn process for starting level
  (bind _isstartinglevel (CallFunction|GetIsStartingLevel))
  (if _isstartinglevel
    (CallFunction|SpawnInputReceivers)
    (bind _returnvalue_3 (UserInterface|CreateWidget "/Game/UI/PreGame/WBP_Menu.WBP_Menu_C"))
    (bind _output_get (Variables|Default|SetMenuWidgetRef _returnvalue_3))
    (UserInterface|Viewport|AddtoViewport _output_get 0)
    (else
      ;[0.05127 0.05127 0.05127] Spawn process for any other level
      (CallFunction|SpawnPlayersSkipMenus)
      (CallFunction|StartGame))))

(fn ConstructionScript)

(fn GetPlayerStartPoints
  (bind _outactors (Actor|GetAllActorsOfClass "/Script/Engine.PlayerStart"))
  (Variables|Default|SetPlayerStartArray _outactors))

(fn SpawnInputReceivers
  (for (_ _array_index) (Variables|Default|GetPlayerStartArray)
    (LocalVariables|SetIndex _array_index)
    (for _array_element (Variables|Default|GetPlayerStartArray)
      (if (== (CallFunction|NametoInt _array_element) (LocalVariables|GetIndex))
        (Class|GameplayStatics|CreatePlayer -1)
        (bind _returnvalue (Game|SpawnActorfromClass "/Game/Core/BP_InputReceiver.BP_InputReceiver_C" (Transformation|GetActorTransform (Utilities|Array|Get(acopy) (Variables|Default|GetPlayerStartArray) (LocalVariables|GetIndex))) "Undefined" 0 (LocalVariables|GetIndex) 0))
        (Utilities|Array|AddUnique (Variables|Default|GetPlayerInputReceiverArray) _returnvalue)
        (Pawn|Possess (Game|GetPlayerController (LocalVariables|GetIndex)) _returnvalue)
        (Utilities|Array|AddUnique (Variables|Default|GetPlayerControllerArray) (Game|GetPlayerController (LocalVariables|GetIndex)))
        (Game|Player|SetViewTargetwithBlend (Game|GetPlayerController (LocalVariables|GetIndex)) (Variables|Default|GetCameraRef) 0.0 "VTBlend_Linear" 0.0 false)))
    (CallFunction|RemoveUnusedCameras)))

(fn NametoInt
  (params (PlayerStart :type Player%20Start%20Object%20Reference))
  (return (Math|Conversions|ToInteger(Byte) (Utilities|String|ToString(Name) (Variables|/Script/Engine.PlayerStart|GetPlayerStartTag PlayerStart)))))

(fn GameStarted
  (Variables|Default|SetbIsInGame true)
  (bind _playermap (Class|BPIGameInstance|GetPlayerMap(Message) (Game|GetGameInstance)))
  (Default|GameStarted (Variables|Default|GetCameraRef) _playermap)
  (Variables|Default|GetMenuWidgetRef
    (:then
      (Widget|RemovefromParent (Variables|Default|GetMenuWidgetRef))
      (Variables|Default|SetMenuWidgetRef 0))
    (:else)))

(fn RemoveUnusedCameras
  (bind _outactors (Actor|GetAllActorsOfClass "/Script/Engine.CameraActor"))
  (for _array_element _outactors
    (Actor|DestroyActor _array_element)))

(fn SpawnPlayersSkipMenus
  (bind _playermap (Class|BPIGameInstance|GetPlayerMap(Message) (Game|GetGameInstance)))
  (bind _keys (Utilities|Map|Keys _playermap))
  (for _array_element _keys
    (LocalVariables|SetPlayerIndexLoc _array_element)
    (bind _characterchoice (Class|BPIGameInstance|GetCharacterChoice(Message) (Game|GetGameInstance) (LocalVariables|GetPlayerIndexLoc)))
    (bind _returnvalue (CallFunction|DoCustomSpawn))
    (bind _returnvalue_2 (Game|SpawnActorfromClass "/Game/Characters/BP_Player.BP_Player_C" _returnvalue "Undefined" 0 _characterchoice (LocalVariables|GetPlayerIndexLoc) 0))
    (Class|BPIGameInstance|AddNewPlayer(Message) (Game|GetGameInstance) (LocalVariables|GetPlayerIndexLoc) _returnvalue_2)
    (Pawn|Possess (Game|GetPlayerController (LocalVariables|GetPlayerIndexLoc)) _returnvalue_2)
    (Bindings|BindtoPlayerEvents _returnvalue_2))
  (CallFunction|RemoveUnusedCameras)
  (Class|BPIGameInstance|ExecutedCustomSpawn(Message) (Game|GetGameInstance)))

(fn DoCustomSpawn
  ;[0.05127 0.05127 0.05127] Has a custom spawn tag been set? If there is a player start tag matching the custom spawn tag, spawn the player there
  (bind _array_element (Utilities|Array|ForEachLoopwithBreak (Variables|Default|GetPlayerStartArray) :!label _label)
    (:LoopBody
      (bind _customspawntag (Class|BPIGameInstance|GetCustomSpawnTag(Message) (Game|GetGameInstance)))
      (if (== _customspawntag (Variables|/Script/Engine.PlayerStart|GetPlayerStartTag _array_element))
        (LocalVariables|SetDoCustomSpawn true)
        (LocalVariables|SetSpawnTransform (Transformation|GetActorTransform _array_element))
        (goto _label Break)))
    (:Completed
      (if (LocalVariables|GetDoCustomSpawn)
        (return (LocalVariables|GetSpawnTransform))
        (else
          ;[0.05127 0.05127 0.05127] If not, spawn them at the first spawn location that doesn't start with "Cust_"
          (bind _array_element_2 (Utilities|Array|ForEachLoopwithBreak (Variables|Default|GetPlayerStartArray) :!label _label_2)
            (:LoopBody
              (if (not (Utilities|String|StartsWith (Utilities|String|ToString(Name) (Variables|/Script/Engine.PlayerStart|GetPlayerStartTag _array_element_2)) "Cust_"))
                (LocalVariables|SetSpawnTransform (Transformation|GetActorTransform _array_element_2))
                (goto _label_2 Break)))
            (:Completed
              (return (LocalVariables|GetSpawnTransform)))))))))

(fn BindtoPlayerEvents
  (params (Player :type BP%20Player%20Object%20Reference))
  (EventDispatchers|BindEventtoPlayerDied Player (EventDispatchers|CreateEvent :!event Custom|OnPlayerDied))
  (EventDispatchers|BindEventtoRevivePlayer Player (EventDispatchers|CreateEvent :!event OnPlayerRevived)))

(fn OnPlayerRevived
  (params (PlayerToRevive :type BP%20Player%20Object%20Reference))
  (Variables|Default|SetPlayersDeadCount (- (Variables|Default|GetPlayersDeadCount) 1)))

(fn CallFadeinGameHUD
  (Default|CallFadeinGameHUD)
  (return false))

(fn DisplayCharacterSelect
  (params (CurrentPlayerIndex :type Integer))
  (bind _characterselect (Default|AddCharacterSelect (Variables|Default|GetMenuWidgetRef) CurrentPlayerIndex))
  (Variables|/Game/Core/BP_InputReceiver.BP_InputReceiver_C|SetCharacterMenuRef (Utilities|Array|Get(acopy) (Variables|Default|GetPlayerInputReceiverArray) CurrentPlayerIndex) _characterselect)
  (return false))

(fn GetCamera
  (return (Variables|Default|GetCameraRef)))

(fn GetIsinGame
  (return (Variables|Default|GetbIsInGame)))

(fn GetIsStartingLevel
  (bind _returnvalue (Game|GetCurrentLevelName true))
  (if (or (Utilities|Enum|Equal(Enum) _returnvalue "Level_01") (Utilities|Enum|Equal(Enum) _returnvalue "TestLevel"))
    (Development|PrintString "STARTING LEVEL" false true "(R=1.000000,G=0.000000,B=0.134815,A=1.000000)" 3.0)
    (return true)
    (else
      (Development|PrintString "NOT STARTING LEVEL" false true "(R=1.000000,G=0.000000,B=0.134815,A=1.000000)" 3.0)
      (return false))))

(fn SpawnPlayer
  (params (CurrentPlayerIndex :type Integer) (CharacterChoice :type Integer) (InputReceiver :type BP%20Input%20Receiver%20Object%20Reference))
  (bind _menuwidgetref (Variables|Default|GetMenuWidgetRef)
    (:then
      (Widget|SetVisibility (Variables|/Game/UI/PreGame/WBP_Menu.WBP_Menu_C|GetStartGame_Txt _menuwidgetref) "SelfHitTestInvisible"))
    (:else
      _))
  (bind _returnvalue (Game|SpawnActorfromClass "/Game/Characters/BP_Player.BP_Player_C" (Transformation|GetActorTransform InputReceiver) "Undefined" 0 CharacterChoice CurrentPlayerIndex 0))
  (Class|BPIGameInstance|AddNewPlayer(Message) (Game|GetGameInstance) CurrentPlayerIndex _returnvalue)
  (Pawn|Possess (Game|GetPlayerController CurrentPlayerIndex) _returnvalue)
  (Bindings|BindtoPlayerEvents _returnvalue)
  (return false))

(fn StartGame
  (CallFunction|GameStarted)
  (Variables|Default|GetInGameHUDRef
    (:then
      (return false))
    (:else
      (bind _playermap (Class|BPIGameInstance|GetPlayerMap(Message) (Game|GetGameInstance)))
      (bind _returnvalue (UserInterface|CreateWidget "/Game/UI/InGame/W_InGameHUD.W_InGameHUD_C" 0 _playermap))
      (bind _output_get (Variables|Default|SetInGameHUDRef _returnvalue))
      (UserInterface|Viewport|AddtoViewport _output_get 0)
      (return false))))