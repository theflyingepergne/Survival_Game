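; Core Game Instance Blueprint that holds per-player data and spawn overrides for the game.
; Maps keyed by player index store player references, character choices, and max/current health and stamina, exposed through getter and setter functions.
; A custom spawn tag and flag are set to request a spawn at a tagged player start, then cleared by ExecutedCustomSpawn.
; Player additions and map queries print debug messages.
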(fn AddNewPlayer
  (params (CurrentPlayerIndex :type Integer) (Player :type BP%20Player%20Object%20Reference))
  (Utilities|Map|Add (Variables|Default|GetPlayersMap) CurrentPlayerIndex Player)
  (Development|PrintString (Utilities|String|Append "Added player " (Utilities|String|ToString(Integer) CurrentPlayerIndex)) false true "(R=0.000000,G=0.633680,B=0.114187,A=1.000000)")
  (return false))

(fn ExecutedCustomSpawn
  (Variables|Default|SetCustomSpawnTag "None")
  (Variables|Default|SetDoCustomSpawn false)
  (return false))

(fn GetCharacterChoice
  (params (PlayerIndex :type Integer))
  (return (.Value (Utilities|Map|Find (Variables|Default|GetCharacterChoiceMap) PlayerIndex))))

(fn GetCustomSpawnTag
  (return (Variables|Default|GetCustomSpawnTag)))

(fn GetPlayerHealth
  (params (PlayerIndex :type Integer))
  (return (.Value (Utilities|Map|Find (Variables|Default|GetPlayerHealthMap) PlayerIndex))))

(fn GetPlayerMap
  (bind _playersmap (Variables|Default|GetPlayersMap))
  (bind _keys (Utilities|Map|Keys (Variables|Default|GetPlayersMap)))
  (for _array_element _keys
    (Development|PrintString (Utilities|String|Append "Player " (Utilities|String|ToString(Integer) _array_element)) false true "(R=0.229328,G=0.000000,B=0.543403,A=1.000000)" 5.0))
  (Development|PrintString "Current players: " false true "(R=0.229328,G=0.000000,B=0.543403,A=1.000000)" 5.0)
  (return (Utilities|Map|Length _playersmap) _playersmap))

(fn GetPlayerStamina
  (params (PlayerIndex :type Integer))
  (return (.Value (Utilities|Map|Find (Variables|Default|GetPlayerStaminaMap) PlayerIndex))))

(fn SetCharacterChoice
  (params (PlayerIndex :type Integer) (CharacterChoice :type Integer))
  (Utilities|Map|Add (Variables|Default|GetCharacterChoiceMap) PlayerIndex CharacterChoice)
  (return false))

(fn SetCustomSpawnTag
  (params (PlayerStartTag :type Name :default "None"))
  (bind _output_get (Variables|Default|SetCustomSpawnTag PlayerStartTag))
  (Development|PrintString (Utilities|String|Append "Found custom spawn tag: " (Utilities|String|ToString(Name) _output_get)) false false)
  (Variables|Default|SetDoCustomSpawn true)
  (return false))

(fn SetPlayerHealth
  (params (PlayerIndex :type Integer) (MaxHealth :type Float%20%28double-precision%29) (CurrentHealth :type Float%20%28double-precision%29))
  (Utilities|Map|Add (Variables|Default|GetPlayerHealthMap) PlayerIndex (Utilities|Struct|MakeF_PlayerHealth MaxHealth CurrentHealth))
  (return MaxHealth CurrentHealth))

(fn SetPlayerStamina
  (params (PlayerIndex :type Integer) (MaxStamina :type Float%20%28double-precision%29) (CurrentStamina :type Float%20%28double-precision%29))
  (Utilities|Map|Add (Variables|Default|GetPlayerStaminaMap) PlayerIndex (Utilities|Struct|MakeF_PlayerStamina MaxStamina CurrentStamina))
  (return false))