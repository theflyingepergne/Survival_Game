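; BP_NextLevel is a trigger area that opens the configured next level once every player is inside it.
; On each begin overlap of NextLevelArea, it reads the player map from the game instance through GetPlayerMapMessage.
; It compares the map's entry count with the number of overlapping BP_Player actors and opens the Level reference when the two match.
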(event OnComponentBeginOverlap(NextLevelArea)
  (params (OverlappedComponent :type Primitive%20Component%20Object%20Reference) (OtherActor :type Actor%20Object%20Reference) (OtherComp :type Primitive%20Component%20Object%20Reference) (OtherBodyIndex :type Integer) (bFromSweep :type Boolean) (SweepResult :type Hit%20Result%20Structure%20%28by%20ref%29))
  (bind _playermap (Class|BPIGameInstance|GetPlayerMap(Message) (Game|GetGameInstance)))
  (bind _values (Utilities|Map|Values _playermap))
  (if (== (Utilities|Array|Length _values) (Utilities|Array|Length (Collision|GetOverlappingActors (Variables|Default|GetNextLevelArea) "/Game/Characters/BP_Player.BP_Player_C" :!class /Script/Engine.PrimitiveComponent)))
    (Game|OpenLevel(byObjectReference) (Variables|Default|GetLevel) false)))

(fn ConstructionScript)