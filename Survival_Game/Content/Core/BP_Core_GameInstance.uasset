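; Game instance that holds a registry of players, their character choices and their health stats, all keyed by player index.
; Getter and setter functions wrap three maps, with health stored as a max and current pair in the stats map.
; Adding a player and fetching the player map print debug messages, and the latter also returns the player count.
; The setters return constant default values rather than the stored data.
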(fn AddNewPlayer
  (params (CurrentPlayerIndex :type Integer) (Player :type BP%20Player%20Object%20Reference))
  (Utilities|Map|Add (Variables|Default|GetPlayersMap) CurrentPlayerIndex Player)
  (Development|PrintString (Utilities|String|Append "Added player " (Utilities|String|ToString(Integer) CurrentPlayerIndex)) true true "(R=0.000000,G=0.633680,B=0.114187,A=1.000000)")
  (return false))

(fn GetCharacterChoice
  (params (PlayerIndex :type Integer))
  (return (.Value (Utilities|Map|Find (Variables|Default|GetCharacterChoiceMap) PlayerIndex))))

(fn GetPlayerMap
  (bind _playersmap (Variables|Default|GetPlayersMap))
  (bind _keys (Utilities|Map|Keys (Variables|Default|GetPlayersMap)))
  (for _array_element _keys
    (Development|PrintString (Utilities|String|Append "Player " (Utilities|String|ToString(Integer) _array_element)) true true "(R=0.229328,G=0.000000,B=0.543403,A=1.000000)" 5.0))
  (Development|PrintString "Current players: " true true "(R=0.229328,G=0.000000,B=0.543403,A=1.000000)" 5.0)
  (return (Utilities|Map|Length _playersmap) _playersmap))

(fn GetPlayerStats
  (params (PlayerIndex :type Integer))
  (return (.Value (Utilities|Map|Find (Variables|Default|GetPlayerStatsMap) PlayerIndex))))

(fn SetCharacterChoice
  (params (PlayerIndex :type Integer) (CharacterChoice :type Integer))
  (Utilities|Map|Add (Variables|Default|GetCharacterChoiceMap) PlayerIndex CharacterChoice)
  (return false))

(fn SetHealth
  (params (PlayerIndex :type Integer) (MaxHealth :type Float%20%28double-precision%29) (CurrentHealth :type Float%20%28double-precision%29))
  (Utilities|Map|Add (Variables|Default|GetPlayerStatsMap) PlayerIndex (Utilities|Struct|MakeF_PlayerStats MaxHealth CurrentHealth))
  (return 0.0 0.0))