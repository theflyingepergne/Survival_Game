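; Player controller for a survival game that lets the player open and close the inventory with the Player_Menu input.
; On BeginPlay it casts and caches the survival HUD, then the controlled third-person character and that character's inventory component.
; The input press calls ToggleInventory on the cached component, which is only set if both casts succeed at BeginPlay.
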(event EventBeginPlay
  (bind _assurvival_game_hud (Utilities|Casting|CastToSurvivalGame_HUD (HUD|GetHUD)))
  (Variables|Default|SetAs%20Survival%20Game%20HUD _assurvival_game_hud)
  (bind _asbp_third_person_character (Utilities|Casting|CastToBP_ThirdPersonCharacter (Pawn|GetControlledPawn)))
  (bind _output_get (Variables|Default|SetAs%20BP%20Third%20Person%20Character _asbp_third_person_character))
  (Variables|Default|SetBPC%20Inventory (Variables|/Game/ThirdPerson/Blueprints/BP_ThirdPersonCharacter.BP_ThirdPersonCharacter_C|GetBPC_Inventory _output_get)))

(event Input|ActionEvents|InputActionPlayer_Menu
  (params (Key :type Key%20Structure :default "None"))
  (:Pressed
    (Default|ToggleInventory (Variables|Default|GetBPC%20Inventory))))

(fn ConstructionScript)