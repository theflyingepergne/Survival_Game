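; BP_Core_PlayerState is a core player state Blueprint that holds the player's MaxHealth and CurrentHealth values.
; GetMaxHealth and GetCurrentHealth are plain getters that return those variables.
; BeginPlay prints both values to screen as one concatenated debug string, with no separator or label.
; The graphs contain no logic that changes health, and the construction script is empty.
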(event EventBeginPlay
  (Development|PrintString (Utilities|String|Append (Utilities|String|ToString(Float) (Variables|Default|GetMaxHealth)) (Utilities|String|ToString(Float) (Variables|Default|GetCurrentHealth)))))

(fn ConstructionScript)

(fn GetMaxHealth
  (return (Variables|Default|GetMaxHealth)))

(fn GetCurrentHealth
  (return (Variables|Default|GetCurrentHealth)))