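; Inventory component that creates and toggles the inventory UI for its owning actor.
; On BeginPlay it caches the third-person character and its BP_Core_PC, then adds a W_Inventory linked back to the component to the viewport.
; For non-character owners, the widget is created without caching a controller or setting an owning player.
; ToggleInventory flips widget visibility, switching input mode and mouse cursor through the cached controller.
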(event EventBeginPlay
  (Development|PrintString "inventory init")
  (bind _asbp_third_person_character (Utilities|Casting|CastToBP_ThirdPersonCharacter (Components|GetOwner))
    (:then
      (bind _output_get (Variables|Default|SetAs%20BP%20Third%20Person%20Character _asbp_third_person_character))
      (bind _asbp_core_pc (Utilities|Casting|CastToBP_Core_PC (Pawn|GetController _output_get)))
      (bind _output_get_2 (Variables|Default|SetAs%20BP%20Core%20PC _asbp_core_pc))
      (bind _returnvalue (UserInterface|CreateWidget "/Game/Core/Inventory_System/UI/W_Inventory.W_Inventory_C" _output_get_2 self))
      (bind _output_get_3 (Variables|Default|SetW_Inventory _returnvalue))
      (UserInterface|Viewport|AddtoViewport _output_get_3 0)
      (Development|PrintString "01"))
    (:CastFailed
      (bind _returnvalue_2 (UserInterface|CreateWidget "/Game/Core/Inventory_System/UI/W_Inventory.W_Inventory_C" 0 self))
      (bind _output_get_4 (Variables|Default|SetW_Inventory _returnvalue_2))
      (UserInterface|Viewport|AddtoViewport _output_get_4 0)
      (Development|PrintString "02"))))

(fn ToggleInventory
  (bind _w_inventory (Variables|Default|GetW_Inventory))
  (bind _as_bp_core_pc (Variables|Default|GetAs%20BP%20Core%20PC))
  (bind _as_bp_core_pc_2 (Variables|Default|GetAs%20BP%20Core%20PC))
  (if (Widget|IsVisible (Variables|Default|GetW_Inventory))
    (Widget|SetVisibility (Variables|Default|GetW_Inventory) "Collapsed")
    (Input|SetInputModeGameOnly _as_bp_core_pc_2)
    (Variables|/Script/Engine.PlayerController|SetbShowMouseCursor _as_bp_core_pc_2 false)
    (else
      (Widget|SetVisibility _w_inventory "SelfHitTestInvisible")
      (Input|SetInputModeGameandUI _as_bp_core_pc _w_inventory "DoNotLock" false)
      (Variables|/Script/Engine.PlayerController|SetbShowMouseCursor _as_bp_core_pc true))))