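; Game mode for local multiplayer that runs the menu, character selection and match start on one shared BP_Camera.
; On BeginPlay it creates a player per tag-numbered PlayerStart, each possessing a BP_InputReceiver, and destroys CameraActors.
; Character select links menu panels to receivers, then SpawnPlayer swaps possession to a BP_Player with the chosen character.
; StartGame requires a minimum player count, then hands players to the camera and in-game HUD.
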(event EventBeginPlay
  (bind _outactors (Actor|GetAllActorsOfClass "/Game/Camera/BP_Camera.BP_Camera_C"))
  (Variables|Default|SetCameraRef (Utilities|Array|Get(acopy) _outactors))
  (CallFunction|GetPlayerStartPoints)
  (CallFunction|SpawnInputReceivers)
  (bind _returnvalue (UserInterface|CreateWidget "/Game/UI/PreGame/WBP_Menu.WBP_Menu_C"))
  (bind _output_get (Variables|Default|SetMenuWidgetRef _returnvalue))
  (UserInterface|Viewport|AddtoViewport _output_get 0))

(fn ConstructionScript)

(fn GetPlayerStartPoints
  (bind _outactors (Actor|GetAllActorsOfClass "/Script/Engine.PlayerStart"))
  (Variables|Default|SetPlayerStartArray _outactors))

(fn SpawnInputReceivers
  (for (_ _array_index) (Variables|Default|GetPlayerStartArray)
    (LocalVariables|SetIndex _array_index)
    (for _array_element (Variables|Default|GetPlayerStartArray)
      (if (== (CallFunction|NametoInt _array_element) (LocalVariables|GetIndex))
        (Class|GameplayStatics|CreatePlayer -1)
        (bind _returnvalue (Game|SpawnActorfromClass "/Game/Core/BP_InputReceiver.BP_InputReceiver_C" (Transformation|GetActorTransform (Utilities|Array|Get(acopy) (Variables|Default|GetPlayerStartArray) (LocalVariables|GetIndex))) "Undefined" 0 (LocalVariables|GetIndex) 0))
        (Utilities|Array|AddUnique (Variables|Default|GetPlayerInputReceiverArray) _returnvalue)
        (Pawn|Possess (Game|GetPlayerController (LocalVariables|GetIndex)) _returnvalue)
        (Utilities|Array|AddUnique (Variables|Default|GetPlayerControllerArray) (Game|GetPlayerController (LocalVariables|GetIndex)))
        (Game|Player|SetViewTargetwithBlend (Game|GetPlayerController (LocalVariables|GetIndex)) (Variables|Default|GetCameraRef) 0.0 "VTBlend_Linear" 0.0 false)))
    (CallFunction|RemoveUnusedCameras)))

(fn NametoInt
  (params (PlayerStart :type Player%20Start%20Object%20Reference))
  (return (Math|Conversions|ToInteger(Byte) (Utilities|String|ToString(Name) (Variables|/Script/Engine.PlayerStart|GetPlayerStartTag PlayerStart)))))

(fn GameStarted
  (Variables|Default|SetbIsInGame true)
  (Default|GameStarted (Variables|Default|GetCameraRef) (Variables|Default|GetPlayers))
  (Variables|Default|GetMenuWidgetRef
    (:then
      (Widget|RemovefromParent (Variables|Default|GetMenuWidgetRef))
      (Variables|Default|SetMenuWidgetRef 0)
      (Development|PrintString "Game Started!"))
    (:else)))

(fn RemoveUnusedCameras
  (bind _outactors (Actor|GetAllActorsOfClass "/Script/Engine.CameraActor"))
  (for _array_element _outactors
    (Actor|DestroyActor _array_element)))

(fn DisplayCharacterSelect
  (params (CurrentPlayerIndex :type Integer))
  (bind _characterselect (Default|AddCharacterSelect (Variables|Default|GetMenuWidgetRef) CurrentPlayerIndex))
  (Variables|/Game/Core/BP_InputReceiver.BP_InputReceiver_C|SetCharacterMenuRef (Utilities|Array|Get(acopy) (Variables|Default|GetPlayerInputReceiverArray) CurrentPlayerIndex) _characterselect)
  (return false))

(fn GetIsinGame
  (return (Variables|Default|GetbIsInGame)))

(fn SpawnPlayer
  (params (CurrentPlayerIndex :type Integer) (CharacterChoice :type Integer) (InputReceiver :type BP%20Input%20Receiver%20Object%20Reference))
  (Widget|SetVisibility (Variables|/Game/UI/PreGame/WBP_Menu.WBP_Menu_C|GetStartGame_Txt (Variables|Default|GetMenuWidgetRef)) "SelfHitTestInvisible")
  (bind _returnvalue (Game|SpawnActorfromClass "/Game/Characters/BP_Player.BP_Player_C" (Transformation|GetActorTransform InputReceiver) "Undefined" 0 CharacterChoice 0))
  (Utilities|Array|Add (Variables|Default|GetPlayers) _returnvalue)
  (Pawn|Possess (Game|GetPlayerController CurrentPlayerIndex) _returnvalue)
  (Game|Player|SetViewTargetwithBlend (Game|GetPlayerController CurrentPlayerIndex) (Variables|Default|GetCameraRef) 0.0 "VTBlend_Linear" 0.0 false)
  (return false))

(fn StartGame
  (if (>= (Utilities|Array|Length (Variables|Default|GetPlayers)) (Variables|Default|GetMinimumPlayers))
    (CallFunction|GameStarted)
    (Variables|Default|GetInGameHUDRef
      (:then
        (return false))
      (:else
        (bind _returnvalue (UserInterface|CreateWidget "/Game/UI/InGame/W_InGameHUD.W_InGameHUD_C" 0 (Variables|Default|GetPlayers)))
        (bind _output_get (Variables|Default|SetInGameHUDRef _returnvalue))
        (UserInterface|Viewport|AddtoViewport _output_get 0)
        (return false)))))